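; BP_DataManager records simulated sensor telemetry from BP_SimpleVehicle to timestamped CSV files and reloads the level when the pawn is destroyed.
; BeginPlay slows time dilation and shows BP_MainWidget, which supplies sampling rate, save directory and record/pause state.
; AsyncPhysicsTick gates sampling with a modulo test and DoOnce, writing a header once, then appending vehicle Status rows.
; Stopping recording or ending play rewrites the file without empty lines.
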(event Custom|DestroyedPawn
  ;[1 1 1] ポーン破壊が確認されたら初期位置からリスポーン
  (bind _returnvalue (Game|GetCurrentLevelName true))
  (Game|OpenLevel(byName) (Utilities|String|StringToName _returnvalue)))

(event Custom|CEventRecStop
  (bind _targetui (Variables|Default|GetTargetUI))
  (bind _directorytext (Variables|/Game/BluePrints/DataManagement/BP_MainWidget.BP_MainWidget_C|GetDirectoryText _targetui))
  (bind _returnvalue (Class|EditableTextBox|GetText _directorytext))
  (bind _returnvalue_2 (Utilities|String|ToString(Text) _returnvalue))
  ;[1 1 1] ファイル内の空行を削除
  (Variables|Default|SetLoadedText (.StringArray (Class|VictoryBPFunctionLibrary|LoadStringArrayfromFile (Utilities|String|Append (Variables|Default|GetSaveDirectory) (Variables|Default|GetRecordTime) (Variables|Default|GetFileExpantion)) false)))
  (Utilities|Array|RemoveItem (Variables|Default|GetLoadedText) "")
  (Class|VictoryBPFunctionLibrary|FileIOSaveStringArraytoFile (Variables|Default|GetSaveDirectory) (Utilities|String|Append (Variables|Default|GetRecordTime) (Variables|Default|GetFileExpantion)) (Variables|Default|GetLoadedText) true false)
  (Utilities|FlowControl|DoOnce false) ; enters at Reset
)

(event Custom|CEventRecStart
  (bind _output (CallFunction|MakeDateStringNow))
  (Variables|Default|SetRecordTime _output)
  (bind _output_get (Variables|Default|SetSaveDirectory (Utilities|String|ToString(Text) (Variables|/Script/UMG.EditableTextBox|GetText (Variables|/Game/BluePrints/DataManagement/BP_MainWidget.BP_MainWidget_C|GetDirectoryText (Variables|Default|GetTargetUI))))))
  (Development|PrintString _output_get))

(event EventBeginPlay
  (bind _returnvalue (Game|GetPlayerController 0))
  (Variables|Default|SetPlayerStartPosition (Transformation|GetActorTransform (Game|Player|GetPlayerPawn 0)))
  (Utilities|Time|SetGlobalTimeDilation 0.3)
  ;[1 1 1] UIの表示
  (bind _returnvalue_2 (UserInterface|CreateWidget "/Game/BluePrints/DataManagement/BP_MainWidget.BP_MainWidget_C" _returnvalue))
  (bind _output_get (Variables|Default|SetTargetUI _returnvalue_2))
  (UserInterface|Viewport|AddtoViewport _output_get 0)
  (Variables|/Script/Engine.PlayerController|SetbShowMouseCursor _returnvalue true)
  (bind _asbp_simple_vehicle (Utilities|Casting|CastToBP_SimpleVehicle (Game|Player|GetPlayerPawn 0)))
  (Variables|Default|SetAs%20BP%20Simple%20Vehicle _asbp_simple_vehicle))

(event EventAsyncPhysicsTick
  (params (DeltaSeconds :type Float%20%28single-precision%29) (SimSeconds :type Float%20%28single-precision%29))
  (bind _targetui (Variables|Default|GetTargetUI))
  (bind _targetui_2 (Variables|Default|GetTargetUI))
  (bind _targetui_3 (Variables|Default|GetTargetUI))
  (bind _targetui_4 (Variables|Default|GetTargetUI))
  (bind _directorytext (Variables|/Game/BluePrints/DataManagement/BP_MainWidget.BP_MainWidget_C|GetDirectoryText _targetui))
  (bind _directorytext_2 (Variables|/Game/BluePrints/DataManagement/BP_MainWidget.BP_MainWidget_C|GetDirectoryText _targetui_3))
  (bind _hz (Variables|/Game/BluePrints/DataManagement/BP_MainWidget.BP_MainWidget_C|GetHz _targetui_4))
  (bind _returnvalue (Class|EditableTextBox|GetText _directorytext))
  (bind _returnvalue_2 (Class|EditableTextBox|GetText _hz))
  (bind _returnvalue_3 (Class|EditableTextBox|GetText _directorytext_2))
  (bind _returnvalue_4 (Class|VictoryBPFunctionLibrary|TexttoFloat _returnvalue_2))
  (bind _returnvalue_5 (Utilities|String|ToString(Text) _returnvalue))
  (bind _returnvalue_6 (Utilities|String|ToString(Text) _returnvalue_3))
  (bind _returnvalue_7 (/ 1.0 _returnvalue_4))
  ;[1 1 1] 記録タイミング判定
  (if (<= (Math|Float|%(Float) SimSeconds _returnvalue_7) (/ _returnvalue_7 2.0))
    (Utilities|FlowControl|DoOnce true :!label _label
      (:Completed
        (if (Math|Boolean|ANDBoolean (Variables|/Game/BluePrints/DataManagement/BP_MainWidget.BP_MainWidget_C|GetIsRecoding _targetui_2) (not (Variables|/Game/BluePrints/DataManagement/BP_MainWidget.BP_MainWidget_C|GetIsPaused _targetui_2)) (Variables|Default|GetIsPawnHere))
          (Utilities|FlowControl|Sequence
            (:then_0
              (bind (_heder _datastring) (CallFunction|MakeDataString (Variables|/Game/BluePrints/Vheicle/BP_SimpleVehicle.BP_SimpleVehicle_C|GetStatus (Variables|Default|GetAs%20BP%20Simple%20Vehicle))))
              (Utilities|FlowControl|Sequence
                (:then_0
                  (Utilities|FlowControl|DoOnce false
                    (:Completed
                      ;[1 1 1] CSV用のヘッダを作成
                      (Variables|Default|SetLoadedText (Utilities|Array|MakeArray _heder))
                      (Variables|Default|SetSaveDirectory _returnvalue_5)
                      (Class|VictoryBPFunctionLibrary|FileIOSaveStringArraytoFile _returnvalue_5 (Utilities|String|Append (Variables|Default|GetRecordTime) (Variables|Default|GetFileExpantion)) (Variables|Default|GetLoadedText) true false))))
                (:then_1
                  (Variables|Default|SetLoadedText (Utilities|Array|MakeArray _datastring)))))
            (:then_1
              ;[1 1 1] CSV用のデータを書き込み
              (Variables|Default|SetSaveDirectory _returnvalue_6)
              (Class|VictoryBPFunctionLibrary|FileIOSaveStringArraytoFile _returnvalue_6 (Utilities|String|Append (Variables|Default|GetRecordTime) (Variables|Default|GetFileExpantion)) (Variables|Default|GetLoadedText) true true)
              (Default|CallEventRecord))))))
    (else
      (goto _label Reset))))

(event EventEndPlay
  (params (EndPlayReason :type EEndPlayReason%20Enum :default "Destroyed"))
  (bind _targetui (Variables|Default|GetTargetUI))
  (bind _directorytext (Variables|/Game/BluePrints/DataManagement/BP_MainWidget.BP_MainWidget_C|GetDirectoryText _targetui))
  (bind _returnvalue (Class|EditableTextBox|GetText _directorytext))
  (bind _returnvalue_2 (Utilities|String|ToString(Text) _returnvalue))
  ;[1 1 1] ファイル内の空行を削除
  (Variables|Default|SetLoadedText (.StringArray (Class|VictoryBPFunctionLibrary|LoadStringArrayfromFile (Utilities|String|Append (Variables|Default|GetSaveDirectory) (Variables|Default|GetRecordTime) (Variables|Default|GetFileExpantion)) false)))
  (Utilities|Array|RemoveItem (Variables|Default|GetLoadedText) "")
  (Class|VictoryBPFunctionLibrary|FileIOSaveStringArraytoFile (Variables|Default|GetSaveDirectory) (Utilities|String|Append (Variables|Default|GetRecordTime) (Variables|Default|GetFileExpantion)) (Variables|Default|GetLoadedText) true false)
  (Utilities|FlowControl|DoOnce false) ; enters at Reset
)

(fn ConstructionScript)

(fn MakeDateStringNow
  (bind _returnvalue (Math|DateTime|Now))
  (bind (_year _month _day _hour _minute _second) (Math|DateTime|BreakDateTime _returnvalue))
  (Utilities|FlowControl|Sequence
    (:then_0
      (LocalVariables|SetYearI _year)
      (LocalVariables|SetMonthI _month)
      (LocalVariables|SetDaysI _day)
      (LocalVariables|SetHourI _hour)
      (LocalVariables|SetMinutesI _minute)
      (LocalVariables|SetSecondI _second))
    (:then_1
      (if (< (LocalVariables|GetMonthI) 10)
        (LocalVariables|SetMonthS (Utilities|String|Append "0" (Utilities|String|ToString(Integer) (LocalVariables|GetMonthI))))
        (else
          (LocalVariables|SetMonthS (Utilities|String|ToString(Integer) (LocalVariables|GetMonthI))))))
    (:then_2
      (if (< (LocalVariables|GetDaysI) 10)
        (LocalVariables|SetDayS (Utilities|String|Append "0" (Utilities|String|ToString(Integer) (LocalVariables|GetDaysI))))
        (else
          (LocalVariables|SetDayS (Utilities|String|ToString(Integer) (LocalVariables|GetDaysI))))))
    (:then_3
      (if (< (LocalVariables|GetHourI) 10)
        (LocalVariables|SetHourS (Utilities|String|Append "0" (Utilities|String|ToString(Integer) (LocalVariables|GetHourI))))
        (else
          (LocalVariables|SetHourS (Utilities|String|ToString(Integer) (LocalVariables|GetHourI))))))
    (:then_4
      (if (< (LocalVariables|GetMinutesI) 10)
        (LocalVariables|SetMinuteS (Utilities|String|Append "0" (Utilities|String|ToString(Integer) (LocalVariables|GetMinutesI))))
        (else
          (LocalVariables|SetMinuteS (Utilities|String|ToString(Integer) (LocalVariables|GetMinutesI))))))
    (:then_5
      (if (< (LocalVariables|GetSecondI) 10)
        (LocalVariables|SetSecondS (Utilities|String|Append "0" (Utilities|String|ToString(Integer) (LocalVariables|GetSecondI))))
        (else
          (LocalVariables|SetSecondS (Utilities|String|ToString(Integer) (LocalVariables|GetSecondI))))))
    (:then_6
      (Development|PrintString (LocalVariables|GetMinuteS))
      (return (Utilities|String|Append (Utilities|String|ToString(Integer) (LocalVariables|GetYearI)) "_" (LocalVariables|GetMonthS) (LocalVariables|GetDayS) "_" (LocalVariables|GetHourS) (LocalVariables|GetMinuteS) (LocalVariables|GetSecondS))))))

(fn MakeDataString
  (params (DataStatus :type Str%20Output%20Single%20Structure))
  (bind (_time _accelaration_x _accelaration_y _accelaration_z _angularvelocity_roll _angularvelocity_pitch _angularvelocity_yaw _magneticforce_x _magneticforce_y _magneticforce_z _groundreflection1 _groundreflection2 _currentvelocity _targetvelocity _revolutioncounter1 _revolutioncounter2 _batteryvoltage _motorcurrent _geomapping _temp1 _temp2) (Utilities|Struct|BreakStrOutputSingle DataStatus))
  (return (Utilities|String|JoinStringArray (Utilities|Array|MakeArray "Time" "Accelaration-x" "Accelaration-y" "Accelaration-z" "AngularVelocity-roll" "AngularVelocity-pitch" "AngularVelocity-yaw" "MagneticForce-x" "MagneticForce-y" "MagneticForce-z" "GroundReflection1" "GroundReflection2" "CurrentVelocity" "TargetVelocity" "RevolutionCounter1" "RevolutionCounter2" "BateryVoltage" "MotorCurrent" "GeoMapping" "Temp1" "Temp2") " ,") (Utilities|String|JoinStringArray (Utilities|Array|MakeArray (Utilities|String|ToString(Float) _time) (Utilities|String|ToString(Float) _accelaration_x) (Utilities|String|ToString(Float) _accelaration_y) (Utilities|String|ToString(Float) _accelaration_z) (Utilities|String|ToString(Float) _angularvelocity_roll) (Utilities|String|ToString(Float) _angularvelocity_pitch) (Utilities|String|ToString(Float) _angularvelocity_yaw) (Utilities|String|ToString(Float) _magneticforce_x) (Utilities|String|ToString(Float) _magneticforce_y) (Utilities|String|ToString(Float) _magneticforce_z) (Utilities|String|ToString(Float) _groundreflection1) (Utilities|String|ToString(Float) _groundreflection2) (Utilities|String|ToString(Float) _currentvelocity) (Utilities|String|ToString(Float) _targetvelocity) (Utilities|String|ToString(Float) _revolutioncounter1) (Utilities|String|ToString(Float) _revolutioncounter2) (Utilities|String|ToString(Float) _batteryvoltage) (Utilities|String|ToString(Float) _motorcurrent) _geomapping (Utilities|String|ToString(Float) _temp1) (Utilities|String|ToString(Float) _temp2)) " ,")))