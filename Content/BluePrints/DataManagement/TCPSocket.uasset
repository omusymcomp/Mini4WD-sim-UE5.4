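; TCP client Blueprint that streams recorded text data from BP_DataManager to a remote socket.
; A delayed Tick polls the manager's ConnectionStatus to connect to its IP and port or disconnect, and connection callbacks write the status back.
; The manager's record event triggers sending the first LoadedText entry as bytes while connected.
; Received messages are read, but the result is unused.
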(event Custom|CEvent%20Disconnection
  (params (ConnectionId :type Integer))
  (Development|PrintString "Lost connection")
  (Variables|Default|SetIsSocketConnected false)
  (Variables|/Game/BluePrints/DataManagement/BP_DataManager.BP_DataManager_C|SetConnectionStatus (Variables|Default|GetAs%20BP%20Data%20Manager) "NewEnumerator2"))

(event Custom|CEvent%20Connection
  (params (ConnectionId :type Integer))
  (Development|PrintString "Connected")
  (Variables|Default|SetIsSocketConnected true)
  (Variables|/Game/BluePrints/DataManagement/BP_DataManager.BP_DataManager_C|SetConnectionStatus (Variables|Default|GetAs%20BP%20Data%20Manager) "NewEnumerator0"))

(event Custom|CEvent%20Recieved
  (params (ConnectionId :type Integer) (Message :type Array%20of%20Bytes))
  (Class|TcpSocketConnection|MessageReadString Message (Utilities|Array|Length Message)))

(event Custom|CEvent%20Tick%20Rec
  (if (Variables|Default|GetIsSocketConnected)
    (Class|TcpSocketConnection|SendData (Variables|Default|GetID) (Class|TcpSocketConnection|ToBytes(String) (Utilities|String|Append (Utilities|Array|Get(acopy) (Variables|/Game/BluePrints/DataManagement/BP_DataManager.BP_DataManager_C|GetLoadedText (Variables|Default|GetAs%20BP%20Data%20Manager))) " 
")))))

(event EventBeginPlay
  (bind _asbp_data_manager (Utilities|Casting|CastToBP_DataManager (Game|GetGameMode)))
  (bind _output_get (Variables|Default|SetAs%20BP%20Data%20Manager _asbp_data_manager))
  (EventDispatchers|BindEventtoEventRecord _output_get (delegate Custom|CEvent%20Tick%20Rec)))

(event EventTick
  (params (DeltaSeconds :type Float%20%28single-precision%29))
  (bind _as_bp_data_manager (Variables|Default|GetAs%20BP%20Data%20Manager))
  (bind _as_bp_data_manager_2 (Variables|Default|GetAs%20BP%20Data%20Manager))
  (Utilities|FlowControl|Delay 0.2)
  (switch Utilities|FlowControl|Switch|SwitchonConnectionStatus (Variables|/Game/BluePrints/DataManagement/BP_DataManager.BP_DataManager_C|GetConnectionStatus (Variables|Default|GetAs%20BP%20Data%20Manager))
    (:NewEnumerator1
      (Development|PrintString (Utilities|String|Append "Connecting " (Variables|/Game/BluePrints/DataManagement/BP_DataManager.BP_DataManager_C|GetIPAddress _as_bp_data_manager) ":" (Utilities|String|ToString(Integer) (Variables|/Game/BluePrints/DataManagement/BP_DataManager.BP_DataManager_C|GetPortNum _as_bp_data_manager))))
      (Utilities|FlowControl|Delay 0.5)
      (bind _connectionid (Class|TcpSocketConnection|Connect (Variables|/Game/BluePrints/DataManagement/BP_DataManager.BP_DataManager_C|GetIPAddress _as_bp_data_manager_2) (Variables|/Game/BluePrints/DataManagement/BP_DataManager.BP_DataManager_C|GetPortNum _as_bp_data_manager_2) (delegate Custom|CEvent%20Disconnection) (delegate Custom|CEvent%20Connection) (delegate Custom|CEvent%20Recieved)))
      (Variables|Default|SetID _connectionid))
    (:NewEnumerator2
      (Utilities|FlowControl|Sequence
        (:then_1
          (Class|TcpSocketConnection|Disconnect (Variables|Default|GetID))
          (Variables|/Game/BluePrints/DataManagement/BP_DataManager.BP_DataManager_C|SetConnectionStatus (Variables|Default|GetAs%20BP%20Data%20Manager) "NewEnumerator2"))))))

(fn ConstructionScript)