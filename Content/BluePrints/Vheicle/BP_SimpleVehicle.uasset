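; Drivable Chaos vehicle pawn that doubles as a simulated sensor rig, working with BP_DataManager from the game mode.
; Throttle comes from Enhanced Input, a fixed-power UI slider through a torque curve, or a signed TCP socket value that also selects forward or reverse.
; Accelerometer, gyro and magnetometer readings fill a Status struct with speed, position, lap and section, on record events or while not recording.
; Debug keys are included.
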(event Custom|CE%20Rec%20Tick
  (bind _returnvalue (Transformation|GetActorLocation))
  (bind (_magx _magy _magz) (Utilities|MagfieldSensor))
  (bind (_x _y _z) (Math|Vector|BreakVector _returnvalue))
  (Utilities|FlowControl|Sequence
    (:then_0
      ;[1 1 1] 各種データ計測
      (Variables|Default|SetValMag (Math|Vector|MakeVector _magx _magy _magz))
      (bind _accelaration (CallFunction|Accelometor))
      (Variables|Default|SetValAcc _accelaration)
      (bind (_rotatervelocity _endtime) (CallFunction|GyroMetor))
      (Variables|Default|SetValRotVelocity _rotatervelocity)
      (Variables|Default|SetOldTimeSecond _endtime))
    (:then_1
      ;[1 1 1] データを格納
      (Utilities|Struct|SetmembersinStrOutputSingle (Variables|Default|Getstatus) (Utilities|String|ToString(Float) (Utilities|Time|GetTimeSeconds)) (Utilities|String|ToString(Float) (.X (Math|Vector|BreakVector (Variables|Default|GetValAcc)))) (Utilities|String|ToString(Float) (.Y (Math|Vector|BreakVector (Variables|Default|GetValAcc)))) (Utilities|String|ToString(Float) (.Z (Math|Vector|BreakVector (Variables|Default|GetValAcc)))) (Utilities|String|ToString(Float) (.Roll (Math|Rotator|BreakRotator (Variables|Default|GetValRotVelocity)))) (Utilities|String|ToString(Float) (.Pitch (Math|Rotator|BreakRotator (Variables|Default|GetValRotVelocity)))) (Utilities|String|ToString(Float) (.Yaw (Math|Rotator|BreakRotator (Variables|Default|GetValRotVelocity)))) (Utilities|String|ToString(Float) (.X (Math|Vector|BreakVector (Variables|Default|GetValMag)))) (Utilities|String|ToString(Float) (.Y (Math|Vector|BreakVector (Variables|Default|GetValMag)))) (Utilities|String|ToString(Float) (.Z (Math|Vector|BreakVector (Variables|Default|GetValMag)))) (Utilities|String|ToString(Float) (/ (Math|Vector|VectorLength (Transformation|GetComponentVelocity (Variables|Character|GetMesh))) 1e+01)) (Variables|Default|Getgeoinfo) (Utilities|String|ToString(Integer) (Variables|Default|GetLapCount)) (Utilities|String|ToString(Integer) (Variables|Default|GetSectionNum)) (Utilities|String|ToString(Float) _x) (Utilities|String|ToString(Float) _y) (Utilities|String|ToString(Float) _z)))))

(event Custom|OtherTick_Event
  (bind _returnvalue (Transformation|GetActorLocation))
  (bind (_magx _magy _magz) (Utilities|MagfieldSensor))
  (bind (_x _y _z) (Math|Vector|BreakVector _returnvalue))
  (if (not (Variables|/Game/BluePrints/DataManagement/BP_DataManager.BP_DataManager_C|GetIsRec (Variables|Default|GetAsDataManager)))
    (Utilities|FlowControl|Sequence
      (:then_0
        ;[1 1 1] 各種データ計測
        (Variables|Default|SetValMag (Math|Vector|MakeVector _magx _magy _magz))
        (bind _accelaration (CallFunction|Accelometor))
        (Variables|Default|SetValAcc _accelaration)
        (bind (_rotatervelocity _endtime) (CallFunction|GyroMetor))
        (Variables|Default|SetValRotVelocity _rotatervelocity)
        (Variables|Default|SetOldTimeSecond _endtime))
      (:then_1
        ;[1 1 1] データを格納
        (Utilities|Struct|SetmembersinStrOutputSingle (Variables|Default|Getstatus) (Utilities|String|ToString(Float) (Utilities|Time|GetTimeSeconds)) (Utilities|String|ToString(Float) (.X (Math|Vector|BreakVector (Variables|Default|GetValAcc)))) (Utilities|String|ToString(Float) (.Y (Math|Vector|BreakVector (Variables|Default|GetValAcc)))) (Utilities|String|ToString(Float) (.Z (Math|Vector|BreakVector (Variables|Default|GetValAcc)))) (Utilities|String|ToString(Float) (.Roll (Math|Rotator|BreakRotator (Variables|Default|GetValRotVelocity)))) (Utilities|String|ToString(Float) (.Pitch (Math|Rotator|BreakRotator (Variables|Default|GetValRotVelocity)))) (Utilities|String|ToString(Float) (.Yaw (Math|Rotator|BreakRotator (Variables|Default|GetValRotVelocity)))) (Utilities|String|ToString(Float) (.X (Math|Vector|BreakVector (Variables|Default|GetValMag)))) (Utilities|String|ToString(Float) (.Y (Math|Vector|BreakVector (Variables|Default|GetValMag)))) (Utilities|String|ToString(Float) (.Z (Math|Vector|BreakVector (Variables|Default|GetValMag)))) (Utilities|String|ToString(Float) (/ (Math|Vector|VectorLength (Transformation|GetComponentVelocity (Variables|Character|GetMesh))) 1e+01)) (Variables|Default|Getgeoinfo) (Utilities|String|ToString(Integer) (Variables|Default|GetLapCount)) (Utilities|String|ToString(Integer) (Variables|Default|GetSectionNum)) (Utilities|String|ToString(Float) _x) (Utilities|String|ToString(Float) _y) (Utilities|String|ToString(Float) _z))))))

(event EventBeginPlay)

(event EventPossessed
  (params (NewController :type Controller%20Object%20Reference))
  (bind _asプレイヤーコントローラー (Utilities|Casting|CastToPlayerController NewController))
  (Input|AddMappingContext (PlayerController|LocalPlayerSubsystems|GetEnhancedInputLocalPlayerSubsystem _asプレイヤーコントローラー) "/Game/BluePrints/Inputs/VehicleInputs.VehicleInputs" 0 "(bIgnoreAllPressedKeysUntilRelease=True,bForceImmediately=False,bNotifyUserSettings=False)")
  (bind _asbp_data_manager (Utilities|Casting|CastToBP_DataManager (Game|GetGameMode)))
  (bind _output_get (Variables|Default|SetAsDataManager _asbp_data_manager))
  (EventDispatchers|BindEventtoEventRecord _output_get (delegate Custom|CE%20Rec%20Tick))
  (Variables|/Game/BluePrints/DataManagement/BP_DataManager.BP_DataManager_C|SetIsPawnHere (Variables|Default|GetAsDataManager) true))

(event Input|KeyboardEvents|C
  (params (Key :type Key%20Structure))
  (:Pressed
    (bind _returnvalue (UserInterface|CreateWidget "/Game/BluePrints/Collisions/WBP_LapTimeDisplay.WBP_LapTimeDisplay_C"))
    (UserInterface|Viewport|AddtoViewport _returnvalue 0)
    (bind _returnvalue_2 (Actor|GetActorOfClass "/Game/BluePrints/Collisions/camera.camera_C"))
    (Game|Player|SetViewTargetwithBlend (Game|GetPlayerController 0) _returnvalue_2 0.0 "VTBlend_Linear" 0.0 false)))

(event Input|KeyboardEvents|2
  (params (Key :type Key%20Structure))
  (:Pressed
    (Development|ExecuteConsoleCommand "p.Vehicle.NextDebugPage" 0)))

(event Input|KeyboardEvents|3
  (params (Key :type Key%20Structure))
  (:Pressed
    (bind _isa (Utilities|FlowControl|FlipFlop)
      (:A
        _)
      (:B
        _))
    (Development|ExecuteConsoleCommand (Utilities|String|ToString(Text) (Utilities|Text|FormatText "p.Vehicle.ShowCom {in1}" 0)) 0)))

(event Input|KeyboardEvents|T
  (params (Key :type Key%20Structure))
  (:Pressed
    (bind (_result _returnvalue) (Class|VictoryBPFunctionLibrary|LoadStringfromFile (Utilities|String|Append (Class|KismetSystemLibrary|GetProjectSavedDirectory) "jsontest.json")))
    (if _returnvalue
      (Development|PrintString _result)
      (else
        (Development|PrintString (Utilities|String|ToString(Boolean) _returnvalue))))))

(event Input|KeyboardEvents|1
  (params (Key :type Key%20Structure))
  (:Released
    (Development|ExecuteConsoleCommand "showdebug vehicle" 0)))

(event Input|KeyboardEvents|T
  (params (Key :type Key%20Structure))
  (:Pressed
    (Development|PrintString (Utilities|String|ToString(Float) (Math|Curves|GetFloatValue "/Game/BluePrints/Vheicle/HyperDash_M1.HyperDash_M1" 4839.0)))))

(event Input|KeyboardEvents|Z
  (params (Key :type Key%20Structure))
  (:Pressed
    (bind _aschaos車輪付き乗り物移動コンポーネント (Utilities|Casting|CastToChaosWheeledVehicleMovementComponent (Variables|Default|GetVehicleMovementComponent))
      (:then
        (Class|ChaosWheeledVehicleMovementComponent|SetMaxEngineTorque _aschaos車輪付き乗り物移動コンポーネント 3e+01))
      (:CastFailed
        (Development|PrintString "Failed")))))

(event Input|KeyboardEvents|4
  (params (Key :type Key%20Structure))
  (:Pressed
    (Development|ExecuteConsoleCommand "slomo 0.01" 0))
  (:Released
    (Development|ExecuteConsoleCommand "slomo 1" 0)))

(event Input|KeyboardEvents|Left
  (params (Key :type Key%20Structure))
  (:Pressed
    (Class|ChaosVehicleMovementComponent|SetThrottleInput (Variables|Default|GetVehicleMovementComponent) 1.0)))

(event Input|KeyboardEvents|G
  (params (Key :type Key%20Structure))
  (:Pressed
    (bind _returnvalue (Class|ChaosVehicleMovementComponent|GetThrottleInput (Variables|Default|GetVehicleMovementComponent)))
    (Development|PrintString (Utilities|String|ToString(Float) _returnvalue))))

(event Input|EnhancedActionEvents|EnhancedInputActionInputOpenThrottle
  (params (ActionValue :type Float%20%28double-precision%29) (ElapsedSeconds :type Float%20%28double-precision%29) (TriggeredSeconds :type Float%20%28double-precision%29) (InputAction :type Input%20Action%20Object%20Reference :default "/Game/BluePrints/Inputs/InputOpenThrottle.InputOpenThrottle"))
  (:Triggered
    ;[1 1 1] OFFなら入力に応じて出力変更
    (Class|ChaosVehicleMovementComponent|SetTargetGear (Variables|Default|GetVehicleMovementComponent) 1 true :!label _label) ; ギアをフォワードに入れる
    (if (not (Class|CheckBox|IsChecked (Variables|/Game/BluePrints/DataManagement/BP_MainWidget.BP_MainWidget_C|GetIsPowerFixed (Variables|/Game/BluePrints/DataManagement/BP_DataManager.BP_DataManager_C|GetTargetUI (Variables|Default|GetAsDataManager)))))
      (Class|ChaosVehicleMovementComponent|SetThrottleInput (Variables|Default|GetVehicleMovementComponent) ActionValue)))
  (:Completed
    (goto _label)))

(event Input|EnhancedActionEvents|EnhancedInputActionInputBrake
  (params (ActionValue :type Float%20%28double-precision%29) (ElapsedSeconds :type Float%20%28double-precision%29) (TriggeredSeconds :type Float%20%28double-precision%29) (InputAction :type Input%20Action%20Object%20Reference :default "/Game/BluePrints/Inputs/InputBrake.InputBrake"))
  (bind _vehiclemovementcomponent (Variables|Default|GetVehicleMovementComponent))
  (:Triggered
    (Class|ChaosVehicleMovementComponent|SetBrakeInput _vehiclemovementcomponent ActionValue))
  (:Completed
    (Class|ChaosVehicleMovementComponent|SetBrakeInput _vehiclemovementcomponent ActionValue)))

(event EventTick
  (params (DeltaSeconds :type Float%20%28single-precision%29))
  (bind _vehiclemovementcomponent (Variables|Default|GetVehicleMovementComponent))
  (bind _asdatamanager (Variables|Default|GetAsDataManager))
  (bind _vehiclemovementcomponent_2 (Variables|Default|GetVehicleMovementComponent))
  (bind _targetui (Variables|/Game/BluePrints/DataManagement/BP_DataManager.BP_DataManager_C|GetTargetUI _asdatamanager))
  (CallFunction|OtherTickEvent)
  (if (Class|Pawn|IsPawnControlled)
    (if (not (Variables|/Game/BluePrints/DataManagement/BP_DataManager.BP_DataManager_C|GetIsSocketAllowed _asdatamanager)) ; TCPソケットによる入力の受付
      ;[1 1 1] ONなら出力固定
      (if (Class|CheckBox|IsChecked (Variables|/Game/BluePrints/DataManagement/BP_MainWidget.BP_MainWidget_C|GetIsPowerFixed _targetui)) ; 出力を固定するか？
        (Class|ChaosVehicleMovementComponent|SetTargetGear _vehiclemovementcomponent 1 true)
        (Class|ChaosVehicleMovementComponent|SetThrottleInput _vehiclemovementcomponent (Math|Curves|GetFloatValue (Variables|Default|GetTorqueCurve) (/ (Class|Slider|GetValue (Variables|/Game/BluePrints/DataManagement/BP_MainWidget.BP_MainWidget_C|GetPowerSlider _targetui)) 1e+02)))
        (goto _label Reset)
        (else
          (Utilities|FlowControl|DoOnce false :!label _label
            (:Completed
              (Class|ChaosVehicleMovementComponent|SetThrottleInput (Variables|Default|GetVehicleMovementComponent) 0.0)))))
      (else
        ;[1 1 1] TCPソケットによるスロットル変更
        (if (< (Variables|/Game/BluePrints/DataManagement/BP_DataManager.BP_DataManager_C|GetThrottleBySocket (Variables|Default|GetAsDataManager)) 0.0)
          (Class|ChaosVehicleMovementComponent|SetTargetGear _vehiclemovementcomponent_2 -1 true)
          (else
            (Class|ChaosVehicleMovementComponent|SetTargetGear _vehiclemovementcomponent_2 1 true)))
        (Class|ChaosVehicleMovementComponent|SetThrottleInput (Variables|Default|GetVehicleMovementComponent) (Math|Float|Absolute(Float) (Variables|/Game/BluePrints/DataManagement/BP_DataManager.BP_DataManager_C|GetThrottleBySocket (Variables|Default|GetAsDataManager))))))))

(fn ConstructionScript)

(fn Accelometor
  (LocalVariables|SetAcc (Utilities|World2Local (Utilities|Operators|Divide (- (Transformation|GetComponentVelocity (Variables|Character|GetMesh)) (Variables|Default|GetOldVelocitay)) (- (Utilities|Time|GetTimeSeconds) (Variables|Default|GetOldTimeSecond)) (LocalVariables|GetConstant))))
  (Variables|Default|SetOldVelocitay (Transformation|GetComponentVelocity (Variables|Character|GetMesh)))
  (return (LocalVariables|GetAcc) (Utilities|Time|GetTimeSeconds)))

(fn GyroMetor
  (bind _returnvalue (Utilities|Time|GetTimeSeconds))
  (bind _oldtimesecond (Variables|Default|GetOldTimeSecond))
  (bind _returnvalue_2 (- _oldtimesecond _returnvalue))
  (LocalVariables|SetRotationVelocity (Math|Rotator|MakeRotator (/ (.Roll (Math|Rotator|BreakRotator (Math|Rotator|Delta(Rotator) (Transformation|GetWorldRotation (Variables|Character|GetMesh)) (Variables|Default|GetOldRot)))) _returnvalue_2) (/ (.Pitch (Math|Rotator|BreakRotator (Math|Rotator|Delta(Rotator) (Transformation|GetWorldRotation (Variables|Character|GetMesh)) (Variables|Default|GetOldRot)))) _returnvalue_2) (/ (.Yaw (Math|Rotator|BreakRotator (Math|Rotator|Delta(Rotator) (Transformation|GetWorldRotation (Variables|Character|GetMesh)) (Variables|Default|GetOldRot)))) _returnvalue_2)))
  (Variables|Default|SetOldRot (Transformation|GetWorldRotation (Variables|Character|GetMesh)))
  (return (LocalVariables|GetRotationVelocity) (Utilities|Time|GetTimeSeconds)))